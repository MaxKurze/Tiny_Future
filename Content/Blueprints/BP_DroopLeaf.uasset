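; BP_DroopLeaf is a leaf actor that tilts when the player touches it, then springs them upward.
; Player overlap with its Box restarts a timeline that lerps actor roll toward a drooped angle, keeping the pitch and yaw cached at BeginPlay.
; When the timeline finishes, it launches the player character straight up if they still overlap the Box.
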(event OnComponentBeginOverlap(Box)
  (params (OverlappedComponent :type Primitive%20Component%20Object%20Reference) (OtherActor :type Actor%20Object%20Reference) (OtherComp :type Primitive%20Component%20Object%20Reference) (OtherBodyIndex :type Integer) (bFromSweep :type Boolean) (SweepResult :type Hit%20Result%20Structure%20%28by%20ref%29))
  (bind _initialrotation (Variables|Default|GetInitialRotation))
  (bind (_roll _pitch _yaw) (Math|Rotator|BreakRotator _initialrotation))
  (if (== OtherActor (Game|GetPlayerCharacter 0))
    (bind _newtrack_0 (Timeline|Timeline PlayFromStart)
      (:Update
        (Transformation|SetActorRotation (Math|Rotator|MakeRotator (Math|Float|Lerp 0.0 3e+01 _newtrack_0) _pitch _yaw)))
      (:Finished
        (if (Collision|IsOverlappingActor (Variables|Default|GetBox) (Game|GetPlayerCharacter 0) :!class /Script/Engine.PrimitiveComponent)
          (Character|LaunchCharacter (Game|GetPlayerCharacter 0) "0.000000,0.000000,1500.000000" false false))))))

(event EventBeginPlay
  (Variables|Default|SetInitialRotation (Transformation|GetActorRotation)))

(event Collision|EventActorBeginOverlap
  (params (OtherActor :type Actor%20Object%20Reference)))

(event EventTick
  (params (DeltaSeconds :type Float%20%28single-precision%29)))

(fn ConstructionScript)