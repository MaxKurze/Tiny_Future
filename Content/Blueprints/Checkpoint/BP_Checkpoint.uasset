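; BP_Checkpoint is a checkpoint actor that records itself as the player's current respawn checkpoint.
; When the player character overlaps its Box, it sets CurrentCheckpoint on BP_ThirdPersonCharacter to itself.
; GetRespawnPointWorldTransform builds the respawn transform by adding the RespawnPoint offset to the actor's location, using RespawnPoint's rotation and scale as-is, so actor rotation is not applied.
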(event OnComponentBeginOverlap(Box)
  (params (OverlappedComponent :type Primitive%20Component%20Object%20Reference) (OtherActor :type Actor%20Object%20Reference) (OtherComp :type Primitive%20Component%20Object%20Reference) (OtherBodyIndex :type Integer) (bFromSweep :type Boolean) (SweepResult :type Hit%20Result%20Structure%20%28by%20ref%29))
  (if (== OtherActor (Game|GetPlayerCharacter 0))
    (bind _asbp_third_person_character (Utilities|Casting|CastToBP_ThirdPersonCharacter (Game|GetPlayerCharacter 0)))
    (Variables|/Game/ThirdPerson/Blueprints/BP_ThirdPersonCharacter.BP_ThirdPersonCharacter_C|SetCurrentCheckpoint _asbp_third_person_character self)))

(event EventBeginPlay)

(event Collision|EventActorBeginOverlap
  (params (OtherActor :type Actor%20Object%20Reference)))

(event EventTick
  (params (DeltaSeconds :type Float%20%28single-precision%29)))

(fn ConstructionScript)

(fn GetRespawnPointWorldTransform
  (bind _respawnpoint (Variables|Default|GetRespawnPoint))
  (bind (_location _rotation _scale) (Math|Transform|BreakTransform _respawnpoint))
  (return (Math|Transform|MakeTransform (+ (Transformation|GetActorLocation) _location) _rotation _scale)))