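; WinCondition is a trigger actor that ends play with a win screen when its box is overlapped.
; The box's begin-overlap event creates a widget for the first player, adds it to the viewport, disables that player character's movement and switches input to UI-only focused on the widget.
; The branch condition is hard-wired true, so the overlapping actor is never checked.
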(event OnComponentBeginOverlap(Box)
  (params (OverlappedComponent :type Primitive%20Component%20Object%20Reference) (OtherActor :type Actor%20Object%20Reference) (OtherComp :type Primitive%20Component%20Object%20Reference) (OtherBodyIndex :type Integer) (bFromSweep :type Boolean) (SweepResult :type Hit%20Result%20Structure%20%28by%20ref%29))
  (if true
    (bind _returnvalue (UserInterface|CreateWidget "/Game/Widgets/WinScreen.WinScreen_C" (Game|GetPlayerController 0)))
    (bind _output_get (Variables|Default|SetWinThing _returnvalue))
    (UserInterface|Viewport|AddtoViewport _output_get 0)
    (Pawn|Components|CharacterMovement|DisableMovement (Variables|/Script/Engine.Character|GetCharacterMovement (Game|GetPlayerCharacter 0)))
    (Input|SetInputModeUIOnly (Game|GetPlayerController 0) (Variables|Default|GetWinThing) "DoNotLock" false)))

(event EventBeginPlay)

(event Collision|EventActorBeginOverlap
  (params (OtherActor :type Actor%20Object%20Reference)))

(event EventTick
  (params (DeltaSeconds :type Float%20%28single-precision%29)))

(fn ConstructionScript)